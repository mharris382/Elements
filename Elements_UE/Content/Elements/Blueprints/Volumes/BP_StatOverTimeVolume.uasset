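; Volume actor that periodically applies a configurable gameplay effect, such as damage, to characters inside its box.
; A looping timer at Rate runs on authority only, scanning overlapping actors for living CharacterBase instances with an ability system component.
; It builds a spec from GameplayEffectClass, assigns Amount as the Data.Damage SetByCaller magnitude and applies it to self, printing debug messages.
; The construction script sets the label's text and color.
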(event Custom|Damage%20Tick
  (Networking|SwitchHasAuthority
    (:Authority
      (for _array_element (Collision|GetOverlappingActors (Variables|Default|GetBox) 0 :!class /Script/Engine.PrimitiveComponent)
        (bind _ascharacter_base (Utilities|Casting|CastToCharacterBase _array_element))
        (if (Class|CharacterBase|IsAlive _ascharacter_base)
          (Utilities|IsValid (Ability|GetAbilitySystemComponent _ascharacter_base)
            (:Is%20Valid
              (Ability|GameplayEffect|AssignTagSetbyCallerMagnitude (GameplayEffects|MakeOutgoingSpec (Ability|GetAbilitySystemComponent _ascharacter_base) (Variables|Default|GetGameplayEffectClass) 1.0 (GameplayEffects|MakeEffectContext (Ability|GetAbilitySystemComponent _ascharacter_base))) "(TagName=\"Data.Damage\")" (Variables|Default|GetAmount))
              (GameplayEffects|ApplyGameplayEffectSpecToSelf (Ability|GetAbilitySystemComponent _ascharacter_base) (GameplayEffects|MakeOutgoingSpec (Ability|GetAbilitySystemComponent _ascharacter_base) (Variables|Default|GetGameplayEffectClass) 1.0 (GameplayEffects|MakeEffectContext (Ability|GetAbilitySystemComponent _ascharacter_base))))
              (Development|PrintText "Triggered Damage from Volume"))
            (:Is%20Not%20Valid
              (Development|PrintString (Utilities|String|Append "character " (Utilities|GetDisplayName _ascharacter_base) "is not valid ability system"))))
          (else
            (Development|PrintString (Utilities|String|Append "character " (Utilities|GetDisplayName _ascharacter_base) " is not alive"))))))))

(event EventBeginPlay
  (Utilities|Time|SetTimerbyEvent (delegate Custom|Damage%20Tick) (Variables|Default|GetRate) true))

(event Collision|EventActorBeginOverlap
  (params (OtherActor :type Actor%20Object%20Reference)))

(event EventTick
  (params (DeltaSeconds :type Float%20%28single-precision%29)))

(fn ConstructionScript
  (bind _textrender (Variables|Default|GetTextRender))
  (Rendering|Components|TextRender|SetText _textrender (Variables|Default|GetLabelText))
  (Rendering|Components|TextRender|SetTextRenderColor _textrender (Variables|Default|GetLabelColor)))