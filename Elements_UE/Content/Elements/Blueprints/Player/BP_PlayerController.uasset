(event EventBeginPlay
  (CallFunction|InitHUDRoot))

(event EventTick
  (params (DeltaSeconds :type Float%20%28single-precision%29)))

(event Custom|Init%20HUD%20Root
  (Variables|UI|GetUI%20Root
    (:then)
    (:else
      (bind _returnvalue (UserInterface|CreateWidget "/Game/Elements/UI/WBP_Root.WBP_Root_C" self))
      (bind _output_get (Variables|UI|SetUI%20Root _returnvalue))
      (UserInterface|Viewport|AddtoViewport _output_get 0))))

(event EventPossess
  (params (PossessedPawn :type Pawn%20Object%20Reference))
  (Variables|UI|GetUI%20Root
    (:then
      _)
    (:else
      (CallFunction|InitHUDRoot)))
  (bind _asbp_mage (Utilities|Casting|CastToBP_Mage PossessedPawn))
  (bind _returnvalue (Class|CommonActivatableWidgetContainerBase|AddWidget (Variables|/Game/Elements/UI/WBP_Root.WBP_Root_C|GetStack (Variables|UI|GetUI%20Root)) "/Game/Elements/UI/Elements_HUD.Elements_HUD_C"))
  (Variables|/Game/Elements/UI/Elements_HUD.Elements_HUD_C|SetCharacter _returnvalue _asbp_mage))

(event EventUnPossess
  (params (UnpossessedPawn :type Pawn%20Object%20Reference))
  (Utilities|ClearHUD))

(fn ConstructionScript)