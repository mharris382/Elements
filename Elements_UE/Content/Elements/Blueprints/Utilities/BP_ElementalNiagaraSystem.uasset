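; Niagara component that adapts its effect to a gameplay element, optionally taking the element tag from its owner on BeginPlay.
; SetElement looks up element data, swaps in a per-element override system or the default asset, and sets the element color parameter.
; Helpers spawn the resolved system at a location or attached.
; A flag can skip coloring overrides, though attached spawns always leave overrides uncolored.
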(event EventBeginPlay
  (Variables|Default|SetDefault%20System (AssetData|GetAsset))
  (if (Variables|Default|GetTry%20Get%20Element%20From%20Owner)
    (bind _returnvalue (Class|ElementInterface|GetElementTag(Message) (Components|GetOwner)))
    (CallFunction|SetElement _returnvalue)))

(event EventTick
  (params (DeltaSeconds :type Float%20%28single-precision%29)))

(fn SetElement
  (params (Element :type Gameplay%20Tag%20Structure))
  (bind (_outelementdata _returnvalue) (Class|ElementsBlueprintFunctionLibrary|GetElementDatafromTag self Element))
  (if _returnvalue
    (bind _output_get (Variables|Default|SetElement Element))
    (Variables|Default|SetElement%20Data _outelementdata)
    (bind (_returnvalue_2 _is_override) (Utilities|GetSystemforElement _output_get)
      (:Is%20Valid
        (Class|NiagaraComponent|SetAsset _returnvalue_2 (Variables|Default|GetReset%20Existing%20Override%20Parameters))
        (if (or (not _is_override) (not (Variables|Default|GetDo%20not%20set%20element%20color%20for%20overrides)))
          (Niagara|SetNiagaraVariable(LinearColor) (Variables|Default|GetElement%20Color%20Parameter%20Name) (.ElementColorID (Utilities|Struct|BreakElementData _outelementdata))))))))

(fn SpawnSystematLocation
  (params (Location :type Vector) (Rotation :type Rotator) (Scale :type Vector) (bAutoDestroy :type Boolean) (bAutoActivate :type Boolean) (PoolingMethod :type ENCPoolMethod%20Enum :default "AutoRelease"))
  (bind (_returnvalue _is_override) (Utilities|GetSystemforElement (Variables|Default|GetElement))
    (:Is%20Valid
      (bind _returnvalue_2 (Niagara|SpawnSystematLocation _returnvalue Location Rotation Scale bAutoDestroy bAutoActivate PoolingMethod))
      (if (and (Variables|Default|GetDo%20not%20set%20element%20color%20for%20overrides) _is_override)
        _
        (else
          (Niagara|SetNiagaraVariable(LinearColor) _returnvalue_2 (Variables|Default|GetElement%20Color%20Parameter%20Name) (.elementcolorid (Variables|Default|GetElement%20Data)))))
      (return _returnvalue_2))))

(fn SpawnSystemAttached
  (params (AttachToComponent :type Scene%20Component%20Object%20Reference) (AttachPointName :type Name) (Location :type Vector) (Rotation :type Rotator) (LocationType :type EAttachLocation%20Enum :default "KeepRelativeOffset") (bAutoDestroy :type Boolean) (bAutoActivate :type Boolean) (PoolingMethod :type ENCPoolMethod%20Enum :default "None") (bPreCullCheck :type Boolean))
  (bind (_returnvalue _is_override) (Utilities|GetSystemforElement (Variables|Default|GetElement))
    (:Is%20Valid
      (bind _returnvalue_2 (Niagara|SpawnSystemAttached _returnvalue AttachToComponent AttachPointName Location Rotation LocationType bAutoDestroy bAutoActivate PoolingMethod bPreCullCheck))
      (if _is_override
        _
        (else
          (Niagara|SetNiagaraVariable(LinearColor) _returnvalue_2 (Variables|Default|GetElement%20Color%20Parameter%20Name) (.elementcolorid (Variables|Default|GetElement%20Data)))))
      (return _returnvalue_2))))