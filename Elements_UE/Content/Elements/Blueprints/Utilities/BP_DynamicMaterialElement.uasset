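; Utility Blueprint that tints a mesh with the color of an element identified by gameplay tag.
; SetForMesh creates and caches dynamic material instances for every mesh material, along with the color parameter name.
; SetElement resolves element data via GetElementDataFromTag or an optional manual exact-match scan of DT_ElementData, then applies ElementColorID to those materials.
; SetMeshAndElement chains both steps in one call.
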(event EventBeginPlay)

(event EventTick
  (params (DeltaSeconds :type Float%20%28single-precision%29)))

(fn SetforMesh
  (params (NewParam :type Mesh%20Component%20Object%20Reference) (name :type Name :default "Color"))
  (Utilities|Array|Clear (Variables|Default|GetDynamicMaterials))
  (Utilities|Array|Clear (Variables|Default|GetParamNames))
  (for (_array_element _array_index) (Rendering|Material|GetMaterials NewParam)
    (bind _returnvalue (Rendering|Material|CreateDynamicMaterialInstance NewParam _array_index _array_element "None" :!class /Script/Engine.PrimitiveComponent))
    (Utilities|Array|Add (Variables|Default|GetDynamicMaterials) _returnvalue)
    (Utilities|Array|Add (Variables|Default|GetParamNames) name)))

(fn SetElement
  (params (Tag :type Gameplay%20Tag%20Structure) (manual%20search :type Boolean))
  (if manual%20search
    (LocalVariables|SetPreview%20Found false)
    (bind _outrownames (DataTable|GetDataTableRowNames "/Game/Data/DT_ElementData.DT_ElementData"))
    (bind _array_element (Utilities|Array|ForEachLoopwithBreak _outrownames :!label _label)
      (:LoopBody
        (bind _returnvalue (Utilities|GetDataTableRow "/Game/Data/DT_ElementData.DT_ElementData" _array_element)
          (:then
            (if (GameplayTags|MatchesTag Tag (.ElementTag (Utilities|Struct|BreakElementData _returnvalue)) true)
              (LocalVariables|SetPreview%20Data _returnvalue)
              (LocalVariables|SetPreview%20Found true)
              (goto _label Break)))))
      (:Completed
        (if (LocalVariables|GetPreview%20Found)
          (Variables|Default|SetTag Tag :!label _label_2)
          (for _array_element_2 (Variables|Default|GetDynamicMaterials)
            (Rendering|Material|SetVectorParameterValue _array_element_2 (Utilities|Array|Get(acopy) (Variables|Default|GetParamNames)) (.ElementColorID (Utilities|Struct|BreakElementData (LocalVariables|GetPreview%20Data))) :!class /Script/Engine.MaterialInstanceDynamic)))))
    (else
      (bind (_outelementdata _returnvalue_2) (Class|ElementsBlueprintFunctionLibrary|GetElementDatafromTag self Tag))
      (if _returnvalue_2
        (LocalVariables|SetPreview%20Data _outelementdata)
        (goto _label_2)
        (else
          (Development|PrintText "Tried to set invalid element"))))))

(fn SetMeshandElement
  (params (Tag :type Gameplay%20Tag%20Structure) (Mesh :type Mesh%20Component%20Object%20Reference) (color%20param%20name :type Name) (manual%20search :type Boolean))
  (CallFunction|SetforMesh Mesh color%20param%20name)
  (CallFunction|SetElement Tag manual%20search))