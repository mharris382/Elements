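; A floating stat bar component that displays a configurable Gameplay Ability System attribute of its owning CharacterBase as a fraction of a max-value attribute.
; On BeginPlay it creates a dynamic material instance and starts a looping timer that polls the owner's Ability System Component, rather than using Tick.
; Each update writes the ratio to the material's Fill Percent parameter, hiding the bar if the owner isn't a CharacterBase or either attribute is missing.
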(event Custom|Update%20Bar
  (bind _ascharacter_base (Utilities|Casting|CastToCharacterBase (Components|GetOwner))
    (:then
      (Utilities|IsValid (Ability|GetAbilitySystemComponent _ascharacter_base)
        (:Is%20Valid
          (if (and (.bSuccessfullyFoundAttribute (Ability|Attribute|GetFloatAttributefromAbilitySystemComponent (Ability|GetAbilitySystemComponent _ascharacter_base) (Variables|Default|GetValue%20Attribute))) (.bSuccessfullyFoundAttribute (Ability|Attribute|GetFloatAttributefromAbilitySystemComponent (Ability|GetAbilitySystemComponent _ascharacter_base) (Variables|Default|GetMax%20Value%20Attribute))))
            (Rendering|SetVisibility true false)
            (CallFunction|UpdateMaterial (.ReturnValue (Ability|Attribute|GetFloatAttributefromAbilitySystemComponent (Ability|GetAbilitySystemComponent _ascharacter_base) (Variables|Default|GetValue%20Attribute))) (.ReturnValue (Ability|Attribute|GetFloatAttributefromAbilitySystemComponent (Ability|GetAbilitySystemComponent _ascharacter_base) (Variables|Default|GetMax%20Value%20Attribute))))
            (else
              (Rendering|SetVisibility false false :!label _label))))))
    (:CastFailed
      (goto _label))))

(event EventBeginPlay
  (bind _returnvalue (Rendering|Material|CreateDynamicMaterialInstance 0 (Variables|Default|GetSource%20Material) "None" :!class /Script/Engine.PrimitiveComponent))
  (Variables|Default|SetDynamic%20Material _returnvalue)
  (Utilities|Time|SetTimerbyEvent (delegate Custom|Update%20Bar) 0.1 true))

(event EventTick
  (params (DeltaSeconds :type Float%20%28single-precision%29)))

(fn UpdateMaterial
  (params (Value :type Float%20%28double-precision%29) (Max%20Value :type Float%20%28double-precision%29))
  (Rendering|Material|SetScalarParameterValue (Variables|Default|GetDynamic%20Material) "Fill Percent" (/ Value Max%20Value) :!class /Script/Engine.MaterialInstanceDynamic))