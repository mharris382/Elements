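; Debug actor that prints the matchup between every pair of elements on screen at BeginPlay.
; It gathers element tags from DT_ElementData, then after a short delay queries GetElementRelationship on the element subsystem for every attacker and defender combination, self-pairings included.
; Each result shows as long-lived text, color-coded by whether the attacker is neutral, strong or weak against the defender.
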(event EventBeginPlay
  (bind _outrownames (DataTable|GetDataTableRowNames "/Game/Data/DT_ElementData.DT_ElementData"))
  (for _array_element _outrownames
    (bind _returnvalue (Utilities|GetDataTableRow "/Game/Data/DT_ElementData.DT_ElementData" _array_element)
      (:then
        (Utilities|Array|Add (Variables|Default|GetElements) (.ElementTag (Utilities|Struct|BreakElementData _returnvalue))))))
  (Utilities|FlowControl|Delay 0.2)
  (for _array_element_2 (Variables|Default|GetElements)
    (for _array_element_3 (Variables|Default|GetElements)
      (Utilities|PrintRelationship _array_element_2 _array_element_3))))

(event Collision|EventActorBeginOverlap
  (params (OtherActor :type Actor%20Object%20Reference)))

(event EventTick
  (params (DeltaSeconds :type Float%20%28single-precision%29)))

(fn ConstructionScript)