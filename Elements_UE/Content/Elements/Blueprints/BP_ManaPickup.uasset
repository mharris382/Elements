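; BP_ManaPickup is an elemental mana pickup that applies a GameplayEffect to an eligible Mage on overlap, then destroys itself.
; Pickup runs only on authority, guarded by a PickedUp flag and a CanBePickedUpBy check, and targets the Mage's AbilitySystemComponent.
; SetElementVisuals drives both Niagara effects from element data, called by UpdateElementVisuals and by the construction script, which previews the DT_ElementData row matching ElementTag.
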(event EventBeginPlay
  (bind _returnvalue (Game|GetInstigator))
  (Utilities|IsValid _returnvalue
    (:Is%20Valid
      (bind _ascharacter_base (Utilities|Casting|CastToCharacterBase _returnvalue))
      (Class|ElementInterface|GetElementTag _ascharacter_base))))

(event Collision|EventActorBeginOverlap
  (params (OtherActor :type Actor%20Object%20Reference))
  (Networking|SwitchHasAuthority
    (:Authority
      (if (not (Variables|Default|GetpickedUp))
        (bind _asmage (Utilities|Casting|CastToMage OtherActor))
        (if (Class|ManaPickup|CanbePickedUpby _asmage)
          (Utilities|IsValid (Ability|GetAbilitySystemComponent _asmage)
            (:Is%20Valid
              (Variables|Default|SetpickedUp true)
              (GameplayEffects|ApplyGameplayEffectToSelf :self (Ability|GetAbilitySystemComponent _asmage) :GameplayEffectClass (Variables|ManaPickup|GetGameplayEffect) :Level 1.0)
              (Actor|DestroyActor))))))))

(event EventTick
  (params (DeltaSeconds :type Float%20%28single-precision%29)))

(event EventUpdateElementVisuals
  (params (ElementData :type Element%20Data%20Structure))
  (CallFunction|SetElementVisuals ElementData))

(fn ConstructionScript
  ;[0.08333 0.08333 0.08333 1 45] PReview in Editor Mode
  (LocalVariables|Setpreview%20found false)
  (bind _outrownames (DataTable|GetDataTableRowNames "/Game/Data/DT_ElementData.DT_ElementData"))
  (bind _array_element (Utilities|Array|ForEachLoopwithBreak _outrownames :!label _label)
    (:LoopBody
      (bind _returnvalue (Utilities|GetDataTableRow "/Game/Data/DT_ElementData.DT_ElementData" _array_element)
        (:then
          (if (GameplayTags|MatchesTag (Variables|Default|GetElementTag) (.ElementTag (Utilities|Struct|BreakElementData _returnvalue)) true)
            (LocalVariables|Setpreview%20data _returnvalue)
            (LocalVariables|Setpreview%20found true)
            (goto _label Break)))))
    (:Completed
      (if (LocalVariables|Getpreview%20found)
        (CallFunction|SetElementVisuals (LocalVariables|Getpreview%20data))))))

(fn SetElementVisuals
  (params (ElementData :type Element%20Data%20Structure%20%28by%20ref%29))
  (Effects|Components|ParticleSystem|SetColorParameter (Variables|Default|GetNS_ManaPickup) "Color" (.ElementColorID (Utilities|Struct|BreakElementData ElementData)))
  (Default|SetElement (Variables|Default|GetNS_CollectionEffect) (Variables|Default|GetElementTag)))