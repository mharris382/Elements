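; Enemy projectile aim component that leads a moving character target, preferring the assigned attack target (plus offset) over the parent's target search.
; Each tick it rotates along a suggested launch velocity, with flight time estimated as distance over initial speed.
; Spawn transforms repeat the prediction using the projectile class's speed and gravity, keeping only horizontal direction, or facing the target if prediction fails.
; Debug text and drawing remain enabled.
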(event EventBeginPlay
  (|CallParentFunction))

(event EventTick
  (params (DeltaSeconds :type Float%20%28single-precision%29))
  (bind _returnvalue (Transformation|GetWorldLocation))
  (|CallParentFunction DeltaSeconds)
  (bind (_isfound _targetlocation _targetactor) (CallFunction|GetAimTarget _returnvalue))
  (if _isfound
    (bind _outlaunchvelocity (Class|GameplayStatics|SuggestProjectileVelocityMovingTarget _returnvalue (.AsCharacter%20Base (Utilities|Casting|CastToCharacterBase _targetactor)) (Variables|Default|GetAttackOffset) 0.0 (/ (Math|Vector|Distance(Vector) _targetlocation _returnvalue) (Variables|Default|GetInitialSpeed)) "ForOneFrame"))
    (Transformation|SetWorldRotation (Math|Rotator|MakeRotfromX _outlaunchvelocity) false false)))

(fn GetAimTarget
  (params (Start%20Point :type Vector :default "0, 0, 0"))
  (bind _attacktargetactor (Variables|Default|GetAttackTargetActor))
  (if (Variables|Default|GetHasAttackTarget)
    (return true (+ (Variables|Default|GetAttackOffset) (Transformation|GetActorLocation _attacktargetactor)) _attacktargetactor)
    (else
      (bind (_isfound _targetlocation _targetactor) (|CallParentFunction Start%20Point))
      (return _isfound _targetlocation _targetactor))))

(fn TryGetProjectileSpawnTransformWS
  (params (NewParam :type BP%20Elements%20Projectile%20Class%20Reference))
  (bind _returnvalue (Transformation|GetWorldLocation))
  (bind _returnvalue_2 (Transformation|GetWorldTransform))
  (bind (_stun_effect _element_tag _sphere_radius _default_impact_effect _initial_speed _gravity) (Utilities|GetClassDefaults NewParam))
  (bind _scale (Variables|Default|GetScale))
  (bind _returnvalue_3 (Math|Conversions|ToVector(Float) _scale))
  (bind (_isfound _targetlocation _targetactor) (CallFunction|GetAimTarget _returnvalue))
  (Utilities|IsValid _targetactor
    (:Is%20Valid
      (if _isfound
        (bind _ascharacter_base (Utilities|Casting|CastToCharacterBase _targetactor)
          (:then
            (Development|PrintText (Utilities|Text|FormatText "Initial Speed={0}   GScale = {1}  (Dist={2}/{0}=>Time={3})" _initial_speed _gravity (Math|Vector|Distance(Vector) _targetlocation _returnvalue) (/ (Math|Vector|Distance(Vector) _targetlocation _returnvalue) _initial_speed)))
            (bind (_outlaunchvelocity _returnvalue_4) (Class|GameplayStatics|SuggestProjectileVelocityMovingTarget _returnvalue _ascharacter_base (Variables|Default|GetAttackOffset) _gravity (/ (Math|Vector|Distance(Vector) _targetlocation _returnvalue) _initial_speed) "ForOneFrame"))
            (if _returnvalue_4
              (return true (Math|Transform|MakeTransform _returnvalue (Math|Rotator|FindLookatRotation _returnvalue (+ _returnvalue (* _outlaunchvelocity "1.000000,1.000000,0.000000"))) _returnvalue_3))
              (else
                (return true (Math|Transform|MakeTransform _returnvalue (Math|Rotator|FindLookatRotation _returnvalue _targetlocation) _returnvalue_3)))))
          (:CastFailed
            (return false (Math|Transform|MakeTransform (.location _returnvalue_2) (.rotation _returnvalue_2) (Math|Conversions|ToVector(Float) (Variables|Default|GetScale))))))))
    (:Is%20Not%20Valid
      (return false (Math|Transform|MakeTransform (.location _returnvalue_2) (.rotation _returnvalue_2) (Math|Conversions|ToVector(Float) (Variables|Default|GetScale)))))))