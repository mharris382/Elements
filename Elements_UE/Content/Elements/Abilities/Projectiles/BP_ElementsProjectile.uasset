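; Base elemental ability projectile that takes its element from the instigating character and damages and stuns characters it hits.
; Each tick it sphere-traces from its last frame's location, applying the gameplay effect specs on authority once per living character, excluding the instigator.
; Any trace hit spawns an element-specific Niagara impact, or a default one tinted to the element color, and authority destroys the projectile.
; Child classes can hook UpdateElementVisuals for visuals.
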(event Custom|Update%20Element%20Visuals
  (params (Element :type Gameplay%20Tag%20Structure)))

(event Custom|Spawn%20Impact%20And%20Destroy
  (params (Hit :type Boolean) (NewParam :type Hit%20Result%20Structure))
  (Utilities|FlowControl|Sequence
    (:then_0
      (CallFunction|SpawnImpact Hit NewParam))
    (:then_1
      (Networking|SwitchHasAuthority
        (:Authority
          (Actor|DestroyActor))))))

(event EventBeginPlay
  (Utilities|FlowControl|Sequence
    (:then_0
      (bind _ascharacter_base (Utilities|Casting|CastToCharacterBase (Game|GetInstigator)))
      (bind _returnvalue (Class|CharacterBase|GetCharacterElement _ascharacter_base))
      (CallFunction|SetElement _returnvalue)
      (CallFunction|UpdateElementVisuals (Variables|Default|GetElement%20Tag)))))

(event EventTick
  (params (DeltaSeconds :type Float%20%28single-precision%29))
  (Utilities|FlowControl|Sequence
    (:then_0
      (if (Variables|Default|Gethas%20last%20frame)
        (bind (_outhits _returnvalue) (Collision|MultiSphereTraceForObjects (Variables|Default|Getlast%20frame%20location) (Transformation|GetActorLocation) (Variables|Default|GetSphere%20Radius) (Utilities|Array|MakeArray "ObjectTypeQuery1" "ObjectTypeQuery2" "ObjectTypeQuery3" "ObjectTypeQuery4") false (Utilities|Array|MakeArray (Variables|Default|GetInstigator)) "None"))
        (if _returnvalue
          (Utilities|FlowControl|Sequence
            (:then_0
              (for _array_element _outhits
                (bind _ascharacter_base (Utilities|Casting|CastToCharacterBase (.HitActor (Collision|BreakHitResult _array_element))))
                (Networking|SwitchHasAuthority
                  (:Authority
                    (if (Math|Boolean|ANDBoolean (Class|CharacterBase|IsAlive _ascharacter_base) (!= _ascharacter_base (Game|GetInstigator)) (Utilities|IsValid (Ability|GetAbilitySystemComponent _ascharacter_base)) (not (Utilities|Array|ContainsItem (Variables|Default|GetHit%20Characters) _ascharacter_base)))
                      (Utilities|Array|Add (Variables|Default|GetHit%20Characters) _ascharacter_base)
                      (GameplayEffects|ApplyGameplayEffectSpecToSelf (Ability|GetAbilitySystemComponent _ascharacter_base) (Variables|Default|GetDamageEffectSpecHandle))
                      (GameplayEffects|ApplyGameplayEffectSpecToSelf (Ability|GetAbilitySystemComponent _ascharacter_base) (Variables|Default|GetStun%20Effect)))))))
            (:then_1
              (CallFunction|SpawnImpactandDestroy true (Utilities|Array|Get(acopy) _outhits)))))))
    (:then_1
      (Variables|Default|Setlast%20frame%20location (Transformation|GetActorLocation))
      (Variables|Default|Sethas%20last%20frame true))))

(fn ConstructionScript
  (bind _projectilemovement (Variables|Default|GetProjectileMovement))
  (Variables|/Script/Engine.ProjectileMovementComponent|SetInitialSpeed _projectilemovement (Variables|Default|GetInitial%20Speed))
  (Variables|/Script/Engine.ProjectileMovementComponent|SetProjectileGravityScale _projectilemovement (Variables|Default|GetGravity)))

(fn SetElement
  (params (Tag :type Gameplay%20Tag%20Structure))
  (bind _output_get (Variables|Default|SetElement%20Tag Tag))
  (CallFunction|UpdateElementVisuals _output_get))

(fn SpawnImpact
  (params (InputPin :type Boolean) (Hit :type Hit%20Result%20Structure%20%28by%20ref%29))
  (bind _returnvalue (Transformation|GetActorTransform))
  (bind _element_tag (Variables|Default|GetElement%20Tag))
  (bind _overide_impact_effect (Variables|Default|GetOveride%20Impact%20Effect))
  (bind (_value _returnvalue_2) (Utilities|Map|Find _overide_impact_effect _element_tag))
  (bind _output_get (LocalVariables|Sethit%20sucess InputPin))
  (LocalVariables|Sethit%20result Hit)
  (if _output_get
    _
    (else
      _))
  (bind _returnvalue_3 (Niagara|SpawnSystematLocation (select _returnvalue_2 _value (Variables|Default|GetDefault%20Impact%20Effect)) (select (LocalVariables|Gethit%20sucess) (.Location (Collision|BreakHitResult (LocalVariables|Gethit%20result))) (.location _returnvalue)) (Math|Rotator|SelectRotator (Math|Rotator|MakeRotfromZ (.Normal (Collision|BreakHitResult (LocalVariables|Gethit%20result)))) (.rotation _returnvalue) (LocalVariables|Gethit%20sucess))))
  (if (not _returnvalue_2)
    ;[1 1 1] if we didn't have an element specific impact , set the color of this system to element color
    (bind (_outelementdata _returnvalue_4) (Class|ElementsBlueprintFunctionLibrary|GetElementDatafromTag self (Variables|Default|GetElement%20Tag)))
    (if _returnvalue_4
      (Niagara|SetNiagaraVariable(LinearColor) _returnvalue_3 "Color" (.ElementColorID (Utilities|Struct|BreakElementData _outelementdata))))))

(fn NewFunction)

(fn GetElementTag
  (return (Variables|Default|GetElement%20Tag)))