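; Projectile Blueprint for the Elements Mage, filed under the player basic cast abilities, that colors its mesh by element.
; A dynamic material element component binds the static mesh and element tag to the "Color" parameter in the construction script and again on actor overlap.
; The UpdateElementVisuals event passes a new element to that component, while other behavior is left to the parent class.
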(event EventBeginPlay
  (|CallParentFunction) ; This node is disabled and will not be called.\nDrag off pins to build functionality.
)

(event Collision|EventActorBeginOverlap
  (params (OtherActor :type Actor%20Object%20Reference))
  (|CallParentFunction OtherActor)
  (Default|SetMeshandElement (Variables|Default|GetBP_DynamicMaterialElement) (Variables|Default|GetElement%20Tag) (Variables|Default|GetStaticMesh) "Color" false))

(event EventTick
  (params (DeltaSeconds :type Float%20%28single-precision%29))
  (|CallParentFunction DeltaSeconds))

(event EventUpdateElementVisuals
  (params (Element :type Gameplay%20Tag%20Structure))
  (Default|SetElement (Variables|Default|GetBP_DynamicMaterialElement) Element false))

(fn ConstructionScript
  (|CallParentFunction)
  (Default|SetMeshandElement (Variables|Default|GetBP_DynamicMaterialElement) (Variables|Default|GetElement%20Tag) (Variables|Default|GetStaticMesh) "Color" false))