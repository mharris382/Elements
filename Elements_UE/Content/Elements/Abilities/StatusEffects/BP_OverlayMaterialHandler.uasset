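; BP_OverlayMaterialHandler manages tag-keyed overlay materials on its owning Character's mesh, stored among status effect assets.
; BeginPlay caches the mesh, and SetDynamicMaterialForTag creates one dynamic material instance per gameplay tag, storing it with its opacity parameter name.
; SetOverlayOpacity writes that parameter and applies the instance as the mesh's single overlay.
; A value of zero or below clears the overlay, whichever tag's material is showing.
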(event EventBeginPlay
  (bind _ascharacter (Utilities|Casting|CastToCharacter (Components|GetOwner)))
  (Variables|Default|SetMesh (Variables|/Script/Engine.Character|GetMesh _ascharacter)))

(event EventTick
  (params (DeltaSeconds :type Float%20%28single-precision%29)))

(fn SetDynamicMaterialforTag
  (params (GameplayTag :type Gameplay%20Tag%20Structure) (Parent :type Material%20Interface%20Object%20Reference) (Opacity%20Param%20Name :type Name))
  (LocalVariables|SetNewLocalVar GameplayTag)
  (if (not (.ReturnValue (Utilities|Map|Find (Variables|Default|GetGameplay%20Tag) GameplayTag)))
    (bind _returnvalue (Rendering|Material|CreateDynamicMaterialInstance Parent "None" "None" :!class /Script/Engine.KismetMaterialLibrary))
    (Utilities|Map|Add (Variables|Default|GetGameplay%20Tag) (LocalVariables|GetNewLocalVar) _returnvalue)
    (Utilities|Map|Add (Variables|Default|GetOpacity%20Param%20Name) (LocalVariables|GetNewLocalVar) Opacity%20Param%20Name)))

(fn SetOverlayOpacity
  (params (Key :type Gameplay%20Tag%20Structure%20%28by%20ref%29) (Value :type Float%20%28single-precision%29))
  (bind _gameplay_tag (Variables|Default|GetGameplay%20Tag))
  (bind _opacity_param_name (Variables|Default|GetOpacity%20Param%20Name))
  (bind (_value _returnvalue) (Utilities|Map|Find _gameplay_tag Key))
  (bind (_value_2 _returnvalue_2) (Utilities|Map|Find _opacity_param_name Key))
  (if (and _returnvalue _returnvalue_2)
    (if (<= Value 0.0)
      (Rendering|Material|SetOverlayMaterial (Variables|Default|GetMesh) 0 :!class /Script/Engine.MeshComponent)
      (else
        (Rendering|Material|SetScalarParameterValue _value _value_2 Value :!class /Script/Engine.MaterialInstanceDynamic)
        (Rendering|Material|SetOverlayMaterial (Variables|Default|GetMesh) _value :!class /Script/Engine.MeshComponent)))))