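; Camera-based aiming component for the mage's abilities that supplies aim targets and projectile spawn transforms.
; On BeginPlay it caches the owning BP_Mage and its follow camera.
; GetAimTarget line-traces from the camera along its forward vector, deferring to the parent implementation without a valid camera.
; Spawn transforms sit at the component's location, facing the hit point or the camera direction when nothing is hit.
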(event EventBeginPlay
  (bind _asbp_mage (Utilities|Casting|CastToBP_Mage (Components|GetOwner)))
  (Variables|Default|SetMage _asbp_mage)
  (Variables|Default|SetFollow%20Camera (Variables|/Script/Elements_UE.Mage|GetFollowCamera _asbp_mage)))

(event EventTick
  (params (DeltaSeconds :type Float%20%28single-precision%29)))

(fn GetAimTarget
  (params (Start%20Point :type Vector :default "0, 0, 0"))
  (bind _follow_camera (Variables|Default|GetFollow%20Camera)
    (:then
      (bind (_outhit _returnvalue) (Class|KismetSystemLibrary|LineTraceSinglebyProfile (Transformation|GetWorldLocation _follow_camera) (+ (Transformation|GetWorldLocation _follow_camera) (* (Math|Vector|GetForwardVector _follow_camera) 1e+04)) "BlockAll" false 0 "None" true))
      (if _returnvalue
        (return true (.Location (Collision|BreakHitResult _outhit)) (.HitActor (Collision|BreakHitResult _outhit)))
        (else
          (return false "0, 0, 0" 0))))
    (:else
      (bind (_isfound _targetlocation _targetactor) (|CallParentFunction Start%20Point))
      (return _isfound _targetlocation _targetactor))))

(fn TryGetProjectileSpawnTransformWS
  (params (NewParam :type BP%20Elements%20Projectile%20Class%20Reference))
  (bind _returnvalue (Transformation|GetWorldLocation))
  (bind (_isfound _targetlocation) (CallFunction|GetAimTarget _returnvalue))
  (if _isfound
    (return true (Math|Transform|MakeTransform _returnvalue (Math|Rotator|FindLookatRotation _returnvalue _targetlocation)))
    (else
      (return true (Math|Transform|MakeTransform _returnvalue (Transformation|GetWorldRotation (Variables|Default|GetFollow%20Camera)))))))