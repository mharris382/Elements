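; Gameplay ability that switches the mage avatar to its next element.
; On activation it casts the avatar to BP_Mage, commits, waits one second, calls SwitchNextElement and ends, cancelling if the cast or commit fails.
; A Completed event of IA_ChangeElement repeats the commit, delay and switch sequence without a cancel path.
; Radial menu hover and click events are empty stubs.
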(event Input|EnhancedActionEvents|EnhancedInputActionIA_ChangeElement
  (params (ActionValue :type Boolean) (ElapsedSeconds :type Float%20%28double-precision%29) (TriggeredSeconds :type Float%20%28double-precision%29) (InputAction :type Input%20Action%20Object%20Reference :default "/Game/Elements/Input/Actions/IA_ChangeElement.IA_ChangeElement"))
  (:Completed
    (bind _returnvalue (Ability|CommitAbility))
    (if _returnvalue
      (Utilities|FlowControl|Delay 1.0)
      (Default|SwitchNextElement (stale Ability|EventActivateAbility _asbp_mage))
      (Ability|EndAbility))))

(event Ability|EventActivateAbility
  (bind _asbp_mage (Utilities|Casting|CastToBP_Mage (Ability|GetAvatarActorfromActorInfo))
    (:then
      (bind _returnvalue (Ability|CommitAbility))
      (if _returnvalue
        (Utilities|FlowControl|Delay 1.0)
        (Default|SwitchNextElement _asbp_mage)
        (Ability|EndAbility)
        (else
          (Ability|CancelAbility :!label _label))))
    (:CastFailed
      (goto _label))))

(event Ability|EventOnEndAbility
  (params (bWasCancelled :type Boolean)))

(event EventRadialMenuHoverOver
  (params (RadialMenu :type Object%20Object%20Reference)))

(event EventRadialButtonClick
  (params (RadialMenu :type Object%20Object%20Reference)))