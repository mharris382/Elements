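; Gameplay ability for an area-of-effect attack that spawns an AOE actor at the character's transform or on the floor beneath it.
; After committing, it plays an optional montage and spawns either immediately or on montage completion, cancelling on interruption.
; The actor receives a damage effect spec with set-by-caller magnitude and the caster's element tag, plus damage delay and AI warning settings.
; The ability then ends, optionally leaving the montage playing.
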(event Custom|Try%20End%20Ability
  (if (or (not (Variables|Default|GetWait%20for%20Montage%20to%20Spawn)) (Variables|Default|GetMontage%20Finished))
    (Ability|EndAbility)))

(event Custom|Spawn%20AOE
  (bind _ascharacter_base (Utilities|Casting|CastToCharacterBase (Ability|GetAvatarActorfromActorInfo))
    (:then
      (bind _returnvalue (Ability|GameplayEffect|AssignTagSetbyCallerMagnitude (Ability|MakeOutgoingGameplayEffectSpec (Variables|Default|GetDamageEffect) (Math|Conversions|ToFloat(Integer) (Ability|GetAbilityLevel))) "(TagName=\"Data.Damage\")" (Variables|Default|GetDamage)))
      (bind _returnvalue_2 (Class|CharacterBase|GetCharacterElement _ascharacter_base))
      (bind _returnvalue_3 (Ability|GameplayEffect|AddAssetTag _returnvalue _returnvalue_2))
      (bind _returnvalue_4 (Game|SpawnActorfromClass (Variables|Default|GetAOE%20Class) (Math|Transform|MakeTransform (.Location (Math|Transform|BreakTransform (CallFunction|GetSpawnTransform _ascharacter_base))) (.Rotation (Math|Transform|BreakTransform (CallFunction|GetSpawnTransform _ascharacter_base))) (Math|Conversions|ToVector(Float) (Variables|Default|GetScale))) "AlwaysSpawn" "MultiplyWithRoot" _ascharacter_base _returnvalue_3 _returnvalue_2 _ascharacter_base))
      (Variables|/Game/Elements/Abilities/Abilities/Casts/BP_AoE.BP_AoE_C|SetDelay _returnvalue_4 (Variables|Default|GetDamage%20Delay))
      (Variables|/Game/Elements/Abilities/Abilities/Casts/BP_AoE.BP_AoE_C|SetAI%20Warning _returnvalue_4 (Variables|Default|GetAI%20Warning))
      (CallFunction|TryEndAbility))
    (:CastFailed
      (CallFunction|CustomCancel))))

(event Custom|Custom%20Cancel
  (Variables|Default|SetMontage%20Finished true)
  (Ability|CancelAbility))

(event Ability|EventActivateAbility
  (bind _wait_for_montage_to_spawn (Variables|Default|GetWait%20for%20Montage%20to%20Spawn))
  (bind _returnvalue (Ability|CommitAbility))
  (if _returnvalue
    (bind _aoe_montage (Variables|Default|GetAOE%20Montage)
      (:then
        (Variables|Default|SetMontage%20Finished false)
        (|PlayMontageandWaitProxy "None" _aoe_montage 2.0 "None" (not (Variables|Default|GetWait%20for%20Montage%20to%20End%20Ability)) 1.0 0.0 false
          (:then
            (if (not _wait_for_montage_to_spawn)
              (CallFunction|SpawnAOE :!label _label)))
          (:OnCompleted
            (Variables|Default|SetMontage%20Finished true)
            (if _wait_for_montage_to_spawn
              (goto _label)))
          (:OnInterrupted
            (CallFunction|CustomCancel :!label _label_2))
          (:OnCancelled
            (goto _label_2))))
      (:else
        (Variables|Default|SetMontage%20Finished true)
        (CallFunction|SpawnAoE)))
    (else
      (Ability|CancelAbility))))

(event Ability|EventOnEndAbility
  (params (bWasCancelled :type Boolean)))

(fn GetSpawnTransform
  (params (Character :type Character%20Base%20Object%20Reference))
  (return (select (Variables|Default|GetSpawnOnGround) (Math|Transform|MakeTransform (+ (.ImpactPoint (Collision|BreakHitResult (.HitResult (Utilities|Struct|BreakFindFloorResult (Variables|/Script/Engine.CharacterMovementComponent|GetCurrentFloor (Variables|/Script/Engine.Character|GetCharacterMovement Character)))))) "0.000000,0.000000,2.000000") (.rotation (Transformation|GetActorTransform Character))) (Transformation|GetActorTransform Character))))