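; GA_Summon_AOE is a gameplay ability that places its summoned AOE attack at the target supplied by the avatar's EnemyAimProvider component.
; Activation caches that component, runs the parent activation and immediately ends the ability, or cancels if the component is missing.
; The GetSpawnTransform override passes a CharacterBase target to the parent calculation, uses other targets' actor transforms directly, and falls back to the supplied character without a target.
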(event Ability|EventActivateAbility
  (bind _returnvalue (Ability|GetAvatarActorfromActorInfo))
  (bind _enemyaimprovider (Variables|Default|GetEnemyAimProvider))
  (bind _returnvalue_2 (Actor|GetComponentbyClass _returnvalue _enemyaimprovider))
  (Utilities|IsValid _returnvalue_2
    (:Is%20Valid
      (Variables|Default|SetAim%20Handler _returnvalue_2)
      (|CallParentFunction)
      (Ability|EndAbility))
    (:Is%20Not%20Valid
      (Ability|CancelAbility))))

(event Ability|EventOnEndAbility
  (params (bWasCancelled :type Boolean))
  (|CallParentFunction bWasCancelled) ; This node is disabled and will not be called.\nDrag off pins to build functionality.
)

(fn GetSpawnTransform
  (params (Character :type Character%20Base%20Object%20Reference))
  (bind _aim_handler (Variables|Default|GetAim%20Handler))
  (bind (_target _success) (Default|GetTargetActor _aim_handler))
  (if _success
    (bind _ascharacter_base (Utilities|Casting|CastToCharacterBase _target)
      (:then
        (return (|CallParentFunction _ascharacter_base)))
      (:CastFailed
        (return (Transformation|GetActorTransform _target))))
    (else
      (return (|CallParentFunction Character)))))