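; Gameplay ability that toggles the owning avatar's walking state.
; On activation it checks the avatar's ability system component for the State.Walking tag, applying a walking-off effect if present or a walking effect otherwise.
; It removes or adds replicated loose gameplay tags to match, then ends immediately, so the state persists outside the ability.
; Leftover move-speed debug print and effect nodes are disconnected.
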(event Ability|EventActivateAbility
  (bind _returnvalue (Ability|GetAvatarActorfromActorInfo))
  (if (GameplayTags|HasMatchingGameplayTag (Ability|GetAbilitySystemComponent _returnvalue) "(TagName=\"State.Walking\")")
    (Ability|ApplyGameplayEffectToOwner (Variables|Default|GetWalkingOffEffect))
    (Ability|GameplayEffect|RemoveLooseGameplayTags _returnvalue (Variables|Default|GetGameplay%20Tags) true)
    (else
      (Ability|ApplyGameplayEffectToOwner (Variables|Default|GetWalkingEffect))
      (Ability|GameplayEffect|AddLooseGameplayTags _returnvalue (Variables|Default|GetGameplay%20Tags) true)))
  (Ability|EndAbility))

(event Ability|EventOnEndAbility
  (params (bWasCancelled :type Boolean)))