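; Gameplay ability scaffold for spells, apparently meant to be driven by montage events.
; After committing, it caches the avatar's character and mesh, then immediately registers one-shot waits for Begin, Commit, Activate, Deactivate and Finish event tags.
; Each event routes to a stub handler; montage playback is unwired.
; OnSpellFinished ends the ability, though nothing here calls it, and ending clears all stored wait tasks.
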(event Custom|On%20Event%20Spell%20Finished
  ;[0.2656 0.2656 0.2656 0.5 25] On Ability End
  ;;[0.3767 0.3767 0.3767 0.5] Finish & Cleanup
  (Ability|EndAbility))

(event Ability|EventActivateAbility
  (bind _returnvalue (Ability|CommitAbility))
  (if _returnvalue
    (bind _ascharacter_base (Utilities|Casting|CastToCharacterBase (Ability|GetAvatarActorfromActorInfo))
      (:then
        (bind _output_get (Variables|Default|SetCharacter%20Base _ascharacter_base))
        (bind _output_get_2 (Variables|Default|SetCharacter%20Mesh (Variables|/Script/Engine.Character|GetMesh _output_get)))
        ;[1 0.4878 0.4878 0.492 29] Events
        ;;[1 0.4878 0.4878 0.492 26] Begin
        (bind (_asynctaskproxy _payload) (Ability|Tasks|WaitGameplayEvent "(TagName=\"Event.Spell.Begin\")" 0 true)
          (:then
            (Utilities|Array|Add (Variables|Default|Getwait%20for%20event%20tasks) _asynctaskproxy)
            ;;[1 0.4878 0.4878 0.492 26] Commit
            (bind (_asynctaskproxy_2 _payload_2) (Ability|Tasks|WaitGameplayEvent "(TagName=\"Event.Spell.Commit\")" 0 true)
              (:then
                (Utilities|Array|Add (Variables|Default|Getwait%20for%20event%20tasks) _asynctaskproxy_2)
                ;;[1 0.4878 0.4878 0.492 26] Activate
                (bind (_asynctaskproxy_3 _payload_3) (Ability|Tasks|WaitGameplayEvent "(TagName=\"Event.Spell.Activate\")" 0 true)
                  (:then
                    (Utilities|Array|Add (Variables|Default|Getwait%20for%20event%20tasks) _asynctaskproxy_3)
                    ;;[1 0.4878 0.4878 0.492 26] Deactivate
                    (bind (_asynctaskproxy_4 _payload_4) (Ability|Tasks|WaitGameplayEvent "(TagName=\"Event.Spell.Deactivate\")" 0 true)
                      (:then
                        (Utilities|Array|Add (Variables|Default|Getwait%20for%20event%20tasks) _asynctaskproxy_4)
                        ;;[1 0.4878 0.4878 0.492 26] Finish
                        (bind (_asynctaskproxy_5 _payload_5) (Ability|Tasks|WaitGameplayEvent "(TagName=\"Event.Spell.Finish\")" 0 true)
                          (:then
                            (Utilities|Array|Add (Variables|Default|Getwait%20for%20event%20tasks) _asynctaskproxy_5))
                          (:EventReceived
                            (GameplayEvents|OnSpellEventFinish _payload_5))))
                      (:EventReceived
                        (GameplayEvents|OnSpellEventDeactivate _payload_4))))
                  (:EventReceived
                    (GameplayEvents|OnSpellEventActivate _payload_3))))
              (:EventReceived
                (GameplayEvents|OnSpellEventCommit _payload_2))))
          (:EventReceived
            (GameplayEvents|OnSpellEventBegin _payload))))
      (:CastFailed
        (Ability|EndAbility)))
    (else
      (Ability|EndAbility))))

(event Ability|EventOnEndAbility
  (params (bWasCancelled :type Boolean))
  ;[0.2656 0.2656 0.2656 0.5 25] On Ability End
  (Utilities|CleanupTasks
    (:Completed
      (if bWasCancelled
        _))))

(fn OnSpellEventBegin
  (params (GameplayEventData :type Gameplay%20Event%20Data%20Structure%20%28by%20ref%29))
  (if (GameplayTags|MatchesTag :TagOne (.EventTag (Utilities|Struct|BreakGameplayEventData GameplayEventData)))
    _))

(fn OnSpellEventCommit
  (params (GameplayEventData :type Gameplay%20Event%20Data%20Structure%20%28by%20ref%29))
  (if (GameplayTags|MatchesTag :TagOne (.EventTag (Utilities|Struct|BreakGameplayEventData GameplayEventData)))
    _))

(fn OnSpellEventActivate
  (params (GameplayEventData :type Gameplay%20Event%20Data%20Structure%20%28by%20ref%29))
  (if (GameplayTags|MatchesTag :TagOne (.EventTag (Utilities|Struct|BreakGameplayEventData GameplayEventData)))
    _))

(fn OnSpellEventDeactivate
  (params (GameplayEventData :type Gameplay%20Event%20Data%20Structure%20%28by%20ref%29))
  (if (GameplayTags|MatchesTag :TagOne (.EventTag (Utilities|Struct|BreakGameplayEventData GameplayEventData)))
    _))

(fn OnSpellEventFinish
  (params (GameplayEventData :type Gameplay%20Event%20Data%20Structure%20%28by%20ref%29))
  (if (GameplayTags|MatchesTag :TagOne (.EventTag (Utilities|Struct|BreakGameplayEventData GameplayEventData)))
    _))