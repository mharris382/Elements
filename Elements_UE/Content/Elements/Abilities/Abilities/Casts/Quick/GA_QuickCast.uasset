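; GA_QuickCast is a Gameplay Ability that plays a sped-up cast montage on a CharacterBase avatar.
; Activation is allowed only while the character's movement mode is Walking; the parent's activation check is left disconnected.
; After committing, it plays the montage on the character mesh and ends through CancelAbility on completion, with no handling for interruption.
; A failed commit or invalid avatar also cancels, with debug text printed for avatar errors.
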(event Ability|EventActivateAbility
  (bind _returnvalue (Ability|GetAvatarActorfromActorInfo))
  (Utilities|IsValid _returnvalue
    (:Is%20Valid
      (bind _ascharacter_base (Utilities|Casting|CastToCharacterBase _returnvalue)
        (:then
          (bind _returnvalue_2 (Ability|CommitAbility))
          (if _returnvalue_2
            (Animation|Montage|PlayMontage (Variables|/Script/Engine.Character|GetMesh _ascharacter_base) (Variables|Default|GetCast%20Montage) 2.0
              (:OnCompleted
                (Ability|CancelAbility)))
            (else
              (Ability|CancelAbility :!label _label))))
        (:CastFailed
          (Development|PrintText "GA_QuickCast:  avatar not a character" true true "(R=1.000000,G=0.054274,B=0.000000,A=1.000000)")
          (goto _label))))
    (:Is%20Not%20Valid
      (Development|PrintText "GA_QuickCast:  no avatar set" true true "(R=1.000000,G=0.054274,B=0.000000,A=1.000000)")
      (Ability|CancelAbility))))

(event Ability|EventOnEndAbility
  (params (bWasCancelled :type Boolean)))

(fn K2CanActivateAbility
  (params (ActorInfo :type Gameplay%20Ability%20Actor%20Info%20Structure) (Handle :type Gameplay%20Ability%20Spec%20Handle%20Structure))
  (bind _ascharacter_base (Utilities|Casting|CastToCharacterBase (Ability|GetAvatarActorfromActorInfo))
    (:then
      (if (Utilities|Enum|Equal(Enum) (Variables|/Script/Engine.CharacterMovementComponent|GetMovementMode (Variables|/Script/Engine.Character|GetCharacterMovement _ascharacter_base)) "MOVE_Walking")
        (return "" true)
        (else
          _)))
    (:CastFailed
      _))
  (return "" false))