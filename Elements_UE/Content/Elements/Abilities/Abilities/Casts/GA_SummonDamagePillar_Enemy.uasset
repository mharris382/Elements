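; Enemy gameplay ability that summons a damage area-of-effect actor, named as a damage pillar, at the targeting context.
; After committing, it stores the avatar's enemy target provider component as the aim handler, cancelling if commit fails or the component is missing.
; It starts an optional montage and immediately spawns the AoE without waiting for completion.
; The actor receives a set-by-caller damage effect spec, the caster's element tag and the caster as instigator.
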(event Ability|EventActivateAbility
  (bind _returnvalue (Ability|GetAvatarActorfromActorInfo))
  (bind _returnvalue_2 (Ability|GetAvatarActorfromActorInfo))
  (bind _enemy_target_provider_class (Variables|Default|GetEnemy%20Target%20Provider%20Class))
  (bind _summon_aoe_montage (Variables|Montage|GetSummon%20AoE%20Montage))
  (bind _returnvalue_3 (Actor|GetComponentbyClass _returnvalue _enemy_target_provider_class))
  (bind _ascharacter_base (Utilities|Casting|CastToCharacterBase _returnvalue_2))
  (|CallParentFunction)
  (bind _returnvalue_4 (Ability|CommitAbility))
  (if _returnvalue_4
    (Utilities|IsValid _returnvalue_3
      (:Is%20Valid
        (Variables|Default|SetAim%20Handler _returnvalue_3)
        (Utilities|IsValid _summon_aoe_montage
          (:Is%20Valid
            (|PlayMontageandWaitProxy "None" _summon_aoe_montage (Variables|Montage|GetMontage%20Speed) "None" true 1.0 0.0 false
              (:then
                _)))
          (:Is%20Not%20Valid
            _))
        (bind _target (CallFunction|GetTargetingContext))
        (bind _returnvalue_5 (Ability|GameplayEffect|AssignTagSetbyCallerMagnitude (Ability|MakeOutgoingGameplayEffectSpec (Variables|Default|GetDamage%20Gameplay%20Effect) (Math|Conversions|ToFloat(Integer) (Ability|GetAbilityLevel))) "(TagName=\"Data.Damage\")" (Variables|Default|GetDamage)))
        (|SpawnActor _target (Variables|Default|GetAoE%20Class) _returnvalue_5 (Variables|/Script/Elements_UE.CharacterBase|GetCharacterElementTag _ascharacter_base) _ascharacter_base))
      (:Is%20Not%20Valid
        (Ability|CancelAbility)))
    (else
      (Ability|CancelAbility))))

(event Ability|EventOnEndAbility
  (params (bWasCancelled :type Boolean))
  (|CallParentFunction bWasCancelled) ; This node is disabled and will not be called.\nDrag off pins to build functionality.
)

(fn GetTargetingContext
  (bind _target (|CallParentFunction))
  (return _target))