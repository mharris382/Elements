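; Area-of-effect ability actor with a telegraphed warm-up, then a timed damage window before it destroys itself.
; During warm-up the point light ramps up and, for Mage casters, a sphere trace writes the AoE and avoidance range into nearby enemies' blackboards, immediately for AI.Smart enemies, later for others.
; Afterwards the cylinder damages overlapping characters and the elemental Niagara effect plays.
; Element tag drives visual color; actor scale sizes the light.
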(event EventBeginPlay
  (bind _pointlight (Variables|Default|GetPointLight))
  (Variables|Default|Sett 0.0)
  (Variables|Default|Setwarming%20up true)
  (Variables|Default|SetMax%20Light%20Intensity (Variables|/Script/Engine.LightComponentBase|GetIntensity _pointlight))
  (Rendering|Components|Light|SetIntensity _pointlight 0.0)
  (Collision|SetCollisionEnabled (Variables|Default|GetCylinder) "NoCollision")
  (Utilities|FlowControl|DelayUntilNextTick)
  (Utilities|FlowControl|Delay (Variables|Default|GetDelay))
  (Variables|Default|Setwarming%20up false)
  (Collision|SetCollisionEnabled (Variables|Default|GetCylinder) "QueryAndPhysics")
  (Components|Activation|Activate (Variables|Default|GetBP_ElementalNiagaraSystem) true)
  (Utilities|FlowControl|Delay (Variables|Default|GetDamage%20Duration))
  (Actor|DestroyActor))

(event Collision|EventActorBeginOverlap
  (params (OtherActor :type Actor%20Object%20Reference))
  (bind _ascharacter_base (Utilities|Casting|CastToCharacterBase OtherActor))
  (Class|ElementalDamageCarrier|TryApplyDamagefromHitResult _ascharacter_base (Collision|MakeHitResult false false 0.0 0.0 (Transformation|GetActorLocation _ascharacter_base) (Transformation|GetActorLocation _ascharacter_base) "0,0,1" "0,0,1" 0 _ascharacter_base (Variables|/Script/Engine.Character|GetCapsuleComponent _ascharacter_base))))

(event EventTick
  (params (DeltaSeconds :type Float%20%28single-precision%29))
  (bind _returnvalue (Transformation|GetActorLocation))
  (bind _returnvalue_2 (Transformation|GetActorScale3D))
  (bind _returnvalue_3 (* (.x _returnvalue_2) 5e+01))
  (bind _returnvalue_4 (+ _returnvalue_3 55.0))
  (if (Variables|Default|Getwarming%20up)
    (Utilities|FlowControl|Sequence
      (:then_0
        (bind _output_get (Variables|Default|Sett (Math|Float|Clamp(Float) (+ (/ DeltaSeconds (/ (Variables|Default|GetDelay) 2.0)) (Variables|Default|Gett)))))
        (Rendering|Components|Light|SetIntensity (Variables|Default|GetPointLight) (Math|Float|Lerp 0.0 (Variables|Default|GetMax%20Light%20Intensity) _output_get)))
      (:then_1
        (Utilities|Casting|CastToMage (Game|GetInstigator))
        (bind _outhits (Collision|MultiSphereTraceForObjects _returnvalue _returnvalue _returnvalue_4 (Utilities|Array|MakeArray "ObjectTypeQuery3") false 0 "None"))
        (for _array_element _outhits
          (bind _asbp_enemy_base (Utilities|Casting|CastToBP_EnemyBase (.HitActor (Collision|BreakHitResult _array_element))))
          (Utilities|IsValid (AI|GetAIController _asbp_enemy_base)
            (:Is%20Valid
              (if (or (> (Variables|Default|Gett) (Variables|Default|GetAI%20Warning)) (GameplayTags|HasMatchingGameplayTag (Ability|GetAbilitySystemComponent _asbp_enemy_base) "(TagName=\"AI.Smart\")"))
                (AI|Components|Blackboard|SetValueasFloat (AI|GetBlackboard (AI|GetAIController _asbp_enemy_base)) (Variables|Default|GetAI%20AoE%20Range%20Name) (+ (Components|Capsule|GetScaledCapsuleRadius (Variables|/Script/Engine.Character|GetCapsuleComponent _asbp_enemy_base)) _returnvalue_4))
                (AI|Components|Blackboard|SetValueasObject (AI|GetBlackboard (AI|GetAIController _asbp_enemy_base)) (Variables|Default|GetAI%20AoE%20Name) self)))))))
    (else
      (Rendering|SetVisibility (Variables|Default|GetPointLight) false false)
      (for _array_element_2 (Collision|GetOverlappingActors (Variables|Default|GetCylinder) "/Script/Elements_UE.CharacterBase" :!class /Script/Engine.PrimitiveComponent)
        (bind _returnvalue_5 (Class|ElementalDamageCarrier|TryApplyDamage _array_element_2))
        (if _returnvalue_5
          (Development|PrintString "hit"))))))

(event EventUpdateElementVisuals
  (params (InElementTag :type Gameplay%20Tag%20Structure) (ElementColor :type Linear%20Color%20Structure))
  (Default|SetElement (Variables|Default|GetBP_ElementalNiagaraSystem) InElementTag)
  (Rendering|Components|Light|SetLightColor (Variables|Default|GetPointLight) ElementColor true))

(fn ConstructionScript
  (bind _pointlight (Variables|Default|GetPointLight))
  (bind _defaultsceneroot (Variables|Default|GetDefaultSceneRoot))
  (bind _returnvalue (Transformation|GetWorldScale _defaultsceneroot))
  (Utilities|FlowControl|Sequence
    (:then_0
      (Default|SetElementColorDirect (Variables|Default|GetBP_ElementalNiagaraSystem) (Variables|Default|GetElementTag)))
    (:then_1
      (Rendering|Lighting|SetAttenuationRadius _pointlight (* (.x _returnvalue) 5e+01))
      (Class|PointLightComponent|SetSourceRadius _pointlight (* (.x _returnvalue) 5e+01)))))