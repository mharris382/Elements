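; Passive gameplay ability that lets a character collect a mana pickup when triggered by a gameplay event.
; The event supplies the pickup as instigator, along with its tags and mana amount.
; If the character is below max mana, a gain effect at character level is applied with the amount as SetByCaller magnitude and the tags as asset tags, then the pickup is destroyed.
; Otherwise the ability cancels, leaving the pickup in place.
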(event Custom|Complete%20Ability%20Success
  (Actor|DestroyActor (Variables|Default|GetPickup))
  (Ability|EndAbility))

(event Ability|EventOnEndAbility
  (params (bWasCancelled :type Boolean)))

(event Ability|EventActivateAbilityFromEvent
  (params (EventData :type Gameplay%20Event%20Data%20Structure%20%28by%20ref%29))
  (bind (_eventtag _instigator _target _optionalobject _optionalobject2 _contexthandle _instigatortags _targettags _eventmagnitude) (Utilities|Struct|BreakGameplayEventData EventData))
  (bind _asmana_pickup (Utilities|Casting|CastToManaPickup _instigator)
    (:then
      (Utilities|IsValid _asmana_pickup
        (:Is%20Valid
          (Variables|Default|SetPickup _asmana_pickup)
          (Variables|Default|SetPickup%20Tags _instigatortags)
          (Variables|Default|SetPickup%20Amount _eventmagnitude)
          (bind _ascharacter_base (Utilities|Casting|CastToCharacterBase (Ability|GetAvatarActorfromActorInfo))
            (:then
              (Variables|Default|SetTarget%20Character _ascharacter_base)
              (if (< (Class|CharacterBase|GetMana _ascharacter_base) (Class|CharacterBase|GetMaxMana _ascharacter_base))
                (bind _returnvalue (Ability|GameplayEffect|AssignTagSetbyCallerMagnitude (Ability|MakeOutgoingGameplayEffectSpec (Variables|Default|GetMana%20Gain%20Effect) (Class|CharacterBase|GetCharacterLevel (Variables|Default|GetTarget%20Character))) "(TagName=\"Data.ManaGain\")" (Variables|Default|GetPickup%20Amount)))
                (bind _returnvalue_2 (Ability|GameplayEffect|AddAssetTags _returnvalue (Variables|Default|GetPickup%20Tags)))
                (GameplayEffects|ApplyGameplayEffectSpecToSelf (Ability|GetAbilitySystemComponent (Variables|Default|GetTarget%20Character)) _returnvalue_2)
                (CallFunction|CompleteAbilitySuccess)
                (else
                  (Ability|CancelAbility :!label _label))))
            (:CastFailed
              (goto _label))))
        (:Is%20Not%20Valid
          (goto _label))))
    (:CastFailed
      (goto _label))))