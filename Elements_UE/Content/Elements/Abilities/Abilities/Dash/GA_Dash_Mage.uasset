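; Mage dash gameplay ability that overrides how the parent dash ability picks its direction and animation montage.
; Direction follows the mage's current movement input, falling back to the parent's direction when there is no input.
; The montage is chosen from a directional set by comparing the dash direction to the follow camera's transform, with the parent's montage as fallback.
; A camera-weighted direction blend remains in the graph but never runs.
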(event Ability|EventActivateAbility
  (|CallParentFunction) ; This node is disabled and will not be called.\nDrag off pins to build functionality.
)

(event Ability|EventOnEndAbility
  (params (bWasCancelled :type Boolean))
  (|CallParentFunction bWasCancelled) ; This node is disabled and will not be called.\nDrag off pins to build functionality.
)

(fn GetDashDirection
  (bind _direction (|CallParentFunction))
  (bind _asbp_mage (Utilities|Casting|CastToBP_Mage (Ability|GetAvatarActorfromActorInfo))
    (:then
      (return (Math|Vector|SelectVector (Variables|/Script/Elements_UE.Mage|GetCurrentMovementInput _asbp_mage) _direction (Variables|/Script/Elements_UE.Mage|GetbHasMovementInput _asbp_mage))))
    (:CastFailed
      (return _direction))))

(fn GetDashMontage
  (params (Dash%20Direction :type Vector :default "0, 0, 0"))
  (bind _asmage (Utilities|Casting|CastToMage (Ability|GetAvatarActorfromActorInfo))
    (:then
      (bind _montage (CallFunction|GetDirectionalMontagefromTransform Dash%20Direction (Transformation|GetWorldTransform (Variables|/Script/Elements_UE.Mage|GetFollowCamera _asmage)) (Variables|Default|GetMontages)))
      (Utilities|IsValid _montage
        (:Is%20Valid
          (return _montage))
        (:Is%20Not%20Valid
          _)))
    (:CastFailed
      _))
  (return (|CallParentFunction Dash%20Direction)))