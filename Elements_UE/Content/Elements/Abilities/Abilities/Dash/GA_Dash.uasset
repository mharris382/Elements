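; Gameplay ability that dashes the avatar, playing a montage alongside a root motion constant force.
; Direction is actor forward or, with UseControlRotationForDirection on a CharacterBase, horizontal velocity falling back to control rotation when still, then scaled and offset.
; Exit velocity either retains prior velocity or follows the dash direction.
; On finish, an optional recovery phase can hold a gameplay effect for RecoveryTime before the ability ends.
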(event Ability|EventActivateAbility
  (bind _direction (CallFunction|GetDashDirection))
  (bind _returnvalue (Ability|CommitAbility))
  (if _returnvalue
    (Variables|Default|SetDash%20Started true)
    ;[0.007165 0.2378 0 1 32] Dasj
    (Default|CallOnDashBegin)
    (bind _asynctaskproxy (|PlayMontageandWaitProxy "None" (Variables|Default|GetDashMontage) 1.0 "None" true 1.0 0.0 false)
      (:then
        (Variables|TaskRefs|SetDash%20Montage%20Async%20Task _asynctaskproxy)
        (bind _asynctaskproxy_2 (Ability|Tasks|ApplyRootMotionConstantForce "None" _direction (Variables|DashSettings|GetBase%20Strength) (Variables|DashSettings|GetBase%20Duration) (Variables|DashSettings|GetIs%20Additive) (Variables|VelocityAfterDash|GetStrength%20Over%20Time) "SetVelocity" (CallFunction|GetDashVelocityonEnd _direction) 0.0 (Variables|DashSettings|GetEnable%20Gravity))
          (:then
            (Variables|TaskRefs|SetRoot%20Motion%20Constant%20Force%20Async%20Task _asynctaskproxy_2))
          (:OnFinish
            (Default|CallOnDashBegin)
            ;[0.7762 0.08944 1 0.524 32] Recovery
            (if (> (Variables|DashRecovery|GetRecoveryTime) 0.0)
              (if (Utilities|IsValidClass (Variables|DashRecovery|GetRecovery%20Gameplay%20Effect))
                (bind _returnvalue_2 (Ability|ApplyGameplayEffectToOwner (Variables|DashRecovery|GetRecovery%20Gameplay%20Effect)))
                (Utilities|FlowControl|Delay (Variables|DashRecovery|GetRecoveryTime))
                (Ability|RemoveGameplayEffectFromOwnerWithHandle _returnvalue_2)
                (else
                  (Utilities|FlowControl|Delay 0.2))))
            (Variables|Default|SetDash%20Started false)
            (Ability|EndAbility)))))
    (else
      (Ability|CancelAbility))))

(event Ability|EventOnEndAbility
  (params (bWasCancelled :type Boolean))
  (if bWasCancelled
    _))

(fn GetDashDirection
  (bind _returnvalue (Ability|GetAvatarActorfromActorInfo))
  (bind (_ascharacter_base _bsuccess) (Utilities|Casting|CastToCharacterBase _returnvalue))
  (bind _returnvalue_2 (Transformation|GetVelocity _ascharacter_base))
  (return (+ (Variables|DashDirection|GetAdd%20to%20Dash%20Direction) (* (Math|Vector|SelectVector (Math|Vector|SelectVector (* _returnvalue_2 "1.000000,1.000000,0.000000") (Math|Rotator|GetRotationXVector (Pawn|GetControlRotation (Pawn|GetController _ascharacter_base) :!class /Script/Engine.Controller)) (> (Class|KismetMathLibrary|VSizeXYSquared _returnvalue_2) 0.0)) (Transformation|GetActorForwardVector _returnvalue) (and _bsuccess (Variables|DashDirection|GetUse%20Control%20Rotation%20for%20Direction))) (Variables|DashDirection|GetDash%20Direction%20Multiplier)))))

(fn GetDashVelocityonEnd
  (params (Dash%20Direction :type Vector))
  (return (Math|Vector|SelectVector (Transformation|GetVelocity (Ability|GetAvatarActorfromActorInfo)) (* Dash%20Direction (Variables|VelocityAfterDash|GetRelative%20Velocity%20After%20Dash)) (Variables|VelocityAfterDash|GetRetain%20Prior%20Velocity%20after%20Dash))))