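; BP_Route is a spline-based route in the enemy navigation elements, holding a current point index and a travel direction.
; IncrementPoints steps the index by the direction, modulo the spline point count, so forward travel loops.
; GetSplinePointAsWorldPosition returns the current point in world space, and ChangeDirection negates the direction.
; The modulo has no explicit handling for negative results when stepping backward past the first point.
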(event Custom|Increment%20Points
  (Variables|Default|Setindex (Math|Integer|%(Integer) (+ (Variables|Default|Getindex) (Variables|Default|Getdirection)) (Spline|GetNumberOfSplinePoints (Variables|Default|GetSpline)))))

(event EventBeginPlay)

(event Collision|EventActorBeginOverlap
  (params (OtherActor :type Actor%20Object%20Reference)))

(event EventTick
  (params (DeltaSeconds :type Float%20%28single-precision%29)))

(fn ConstructionScript)

(fn GetSplinePointasWorldPosition
  (return (Spline|GetLocationatSplinePoint (Variables|Default|GetSpline) (Variables|Default|Getindex) "World")))

(fn ChangeDirection
  (Variables|Default|Setdirection (* (Variables|Default|Getdirection) -1)))