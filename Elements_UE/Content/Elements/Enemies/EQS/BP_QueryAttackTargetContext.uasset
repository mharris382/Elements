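; EQS query context that supplies the location of an enemy's attack target to environment queries.
; It casts the querier actor to AIController and reads the target actor from the blackboard's AttackTargetKey, returning zero if that fails.
; When the querier object is the EQS testing pawn, it returns the PlayerStart location instead and prints a reminder to remove this temporary branch.
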(fn ProvideSingleLocation
  (params (QuerierObject :type Object%20Object%20Reference) (QuerierActor :type Actor%20Object%20Reference))
  (Utilities|Casting|CastToBP_EQS_TestingPawn QuerierObject
    (:then
      (Development|PrintString "Remove this from query context after testing")
      (bind _returnvalue (Actor|GetActorOfClass "/Script/Engine.PlayerStart"))
      (Utilities|IsValid _returnvalue
        (:Is%20Valid
          (return (Transformation|GetActorLocation _returnvalue)))
        (:Is%20Not%20Valid
          (return "0, 0, 0"))))
    (:CastFailed
      (bind _asaicontroller (Utilities|Casting|CastToAIController QuerierActor)
        (:then
          (Utilities|IsValid (AI|Components|Blackboard|GetValueasObject (AI|GetBlackboard _asaicontroller) (Variables|Default|GetAttackTargetKey))
            (:Is%20Valid
              (bind _asactor (Utilities|Casting|CastToActor (AI|Components|Blackboard|GetValueasObject (AI|GetBlackboard _asaicontroller) (Variables|Default|GetAttackTargetKey)))
                (:then
                  (return (Transformation|GetActorLocation _asactor)))
                (:CastFailed
                  _)))
            (:Is%20Not%20Valid
              _))
          (return "0, 0, 0"))
        (:CastFailed
          (return "0, 0, 0"))))))