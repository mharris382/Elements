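; Test component for enemy AI that, when testing is enabled, drives an enemy with a chosen behavior tree, route, ability and attack target.
; SetupAIForTesting starts the tree once, assigns the route, writes ability and target to the blackboard, caches controller and enemy, and returns whether testing is on.
; Tick repeats setup on the cached pair, keeping test values applied.
; The ability index wraps around the class list, and null entries print a warning.
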(event EventBeginPlay)

(event EventTick
  (params (DeltaSeconds :type Float%20%28single-precision%29))
  (bind _controller (Variables|Default|GetController)
    (:then
      (bind _enemy (Variables|Default|GetEnemy)
        (:then
          (CallFunction|SetupAIforTesting _controller _enemy))
        (:else)))
    (:else)))

(fn GetAttackTarget
  (if (Variables|TestAbilities|GetTest%20Abilities)
    (bind _attacktarget (Variables|TestAbilities|GetAttackTarget)
      (:then
        (return _attacktarget true))
      (:else
        (bind _actorattacktarget (Variables|TestAbilities|GetActorAttackTarget)
          (:then
            (return _actorattacktarget true))
          (:else
            (return 0 false)))))
    (else
      (return 0 false))))

(fn GetRoute
  (bind _testroute (Variables|Movement|GetTestRoute)
    (:then
      (return true _testroute))
    (:else
      (return false 0))))

(fn SetupAIforTesting
  (params (EnemyController :type AIC%20Enemy%20Controller%20Object%20Reference) (Enemy :type BP%20Enemy%20Base%20Object%20Reference))
  (LocalVariables|SetNewLocalVar EnemyController)
  (LocalVariables|SetNewLocalVar_0 Enemy)
  (Utilities|FlowControl|Sequence
    (:then_0
      (if (Variables|Default|GetEnable%20Testing)
        (Utilities|FlowControl|Sequence
          (:then_0
            (if (not (Variables|Default|Getis%20running))
              (Variables|Default|Setis%20running true)
              ;[1 1 1] Run Behavior Tree
              (AI|RunBehaviorTree (LocalVariables|GetNewLocalVar) (Variables|Default|GetTestBehavior))
              (Utilities|FlowControl|Sequence)))
          (:then_1
            ;[1 1 1] Setup Route
            (bind (_has_route _testroute) (CallFunction|GetRoute))
            (if _has_route
              (Variables|/Game/Elements/Enemies/Characters/BP_EnemyBase.BP_EnemyBase_C|SetRoute (LocalVariables|GetNewLocalVar_0) _testroute)))
          (:then_2
            ;[1 1 1] Setup Primary Ability
            (bind (_output _found) (CallFunction|GetTestAbility))
            (if _found
              (Class|BlackboardComponent|SetValueasClass (AI|GetBlackboard (LocalVariables|GetNewLocalVar)) (Variables|/Game/Elements/Enemies/AI/AIC_EnemyController.AIC_EnemyController_C|GetPrimaryAbilityName (LocalVariables|GetNewLocalVar)) _output)))
          (:then_3
            ;[1 1 1] Setup Attack Target
            (bind (_target _found_2) (CallFunction|GetAttackTarget))
            (AI|Components|Blackboard|SetValueasBool (AI|GetBlackboard (LocalVariables|GetNewLocalVar)) (Variables|/Game/Elements/Enemies/AI/AIC_EnemyController.AIC_EnemyController_C|GetAttackingName (LocalVariables|GetNewLocalVar)) _found_2)
            (AI|Components|Blackboard|SetValueasObject (AI|GetBlackboard (LocalVariables|GetNewLocalVar)) (Variables|/Game/Elements/Enemies/AI/AIC_EnemyController.AIC_EnemyController_C|GetAttackTargetName (LocalVariables|GetNewLocalVar)) _target))
          (:then_4
            (Variables|Default|SetController (LocalVariables|GetNewLocalVar))
            (Variables|Default|SetEnemy (LocalVariables|GetNewLocalVar_0))))))
    (:then_1
      (return (Variables|Default|GetEnable%20Testing)))))

(fn GetTestAbility
  (bind _testabilityclass (Variables|TestAbilities|GetTestAbilityClass))
  (bind _tested_ability_index (Variables|TestAbilities|GetTested%20Ability%20Index))
  (bind _returnvalue (Utilities|Array|Length _testabilityclass))
  (bind _returnvalue_2 (Math|Integer|%(Integer) _tested_ability_index _returnvalue))
  (bind _output (Utilities|Array|Get(acopy) _testabilityclass _returnvalue_2))
  (if (Utilities|IsValidClass _output)
    (return _output true)
    (else
      (Development|PrintString (Utilities|String|Append "Testing enemy has null ability at index " (Utilities|String|ToString(Integer) _returnvalue_2)))
      (return 0 false))))