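; EQS query context, named for fleeing AoE, that supplies a single location to enemy AI queries.
; For a Character querier, it reads the AttackTargetKey actor from the AIC_EnemyController's blackboard and returns that target's location, not an AoE position.
; EQS testing pawns return their own location, and failed lookups return the world origin.
; Disconnected PlayerStart debug branches remain, one printing "NOT IMPLEMENTED".
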(fn ProvideSingleLocation
  (params (QuerierObject :type Object%20Object%20Reference) (QuerierActor :type Actor%20Object%20Reference))
  (bind _asbp_eqs_testing_pawn (Utilities|Casting|CastToBP_EQS_TestingPawn QuerierObject)
    (:then
      (return (Transformation|GetActorLocation _asbp_eqs_testing_pawn)))
    (:CastFailed
      (bind _ascharacter (Utilities|Casting|CastToCharacter QuerierObject)
        (:then
          (bind _asaic_enemy_controller (Utilities|Casting|CastToAIC_EnemyController (Pawn|GetController _ascharacter))
            (:then
              (Utilities|IsValid (AI|Components|Blackboard|GetValueasObject (AI|GetBlackboard _asaic_enemy_controller) (Variables|Default|GetAttackTargetKey))
                (:Is%20Valid
                  (bind _asactor (Utilities|Casting|CastToActor (AI|Components|Blackboard|GetValueasObject (AI|GetBlackboard _asaic_enemy_controller) (Variables|Default|GetAttackTargetKey)))
                    (:then
                      (return (Transformation|GetActorLocation _asactor)))
                    (:CastFailed
                      _)))
                (:Is%20Not%20Valid
                  _))
              (return "0, 0, 0"))
            (:CastFailed
              _)))
        (:CastFailed
          _))
      (return "0, 0, 0"))))