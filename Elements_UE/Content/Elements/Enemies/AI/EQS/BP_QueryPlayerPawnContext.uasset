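; EQS query context that supplies the player's location to enemy AI environment queries.
; It returns the location of player pawn 0, or the world origin if that pawn is invalid.
; When the querier is the EQS testing pawn, it uses a PlayerStart's location instead and prints a reminder to remove this test branch.
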(fn ProvideSingleLocation
  (params (QuerierObject :type Object%20Object%20Reference) (QuerierActor :type Actor%20Object%20Reference))
  (bind _returnvalue (Game|Player|GetPlayerPawn 0))
  (Utilities|Casting|CastToBP_EQS_TestingPawn QuerierObject
    (:then
      (Development|PrintString "Remove this from query context after testing")
      (bind _returnvalue_2 (Actor|GetActorOfClass "/Script/Engine.PlayerStart"))
      (Utilities|IsValid _returnvalue_2
        (:Is%20Valid
          (return (Transformation|GetActorLocation _returnvalue_2)))
        (:Is%20Not%20Valid
          (return "0, 0, 0"))))
    (:CastFailed
      (Utilities|IsValid _returnvalue
        (:Is%20Valid
          (return (Transformation|GetActorLocation _returnvalue)))
        (:Is%20Not%20Valid
          (return "0, 0, 0"))))))