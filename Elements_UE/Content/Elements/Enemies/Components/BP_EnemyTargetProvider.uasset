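; BP_EnemyTargetProvider supplies an enemy's current attack target, both as a plain actor and as Gameplay Ability System target data.
; SetEnemyAttackTarget stores the target, and both getters return it with a success flag that is false when the target is invalid.
; Both attack range queries, general and per ability tag, are placeholders that return zero.
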(event EventBeginPlay)

(event EventTick
  (params (DeltaSeconds :type Float%20%28single-precision%29)))

(event EventSetEnemyAttackTarget
  (params (AttackTarget :type Actor%20Object%20Reference))
  (Variables|Default|SetTarget AttackTarget))

(fn GetEnemyTarget
  (bind _target (Variables|Default|GetTarget))
  (Utilities|IsValid _target
    (:Is%20Valid
      (return (Ability|TargetData|AbilityTargetDatafromActor _target) true))
    (:Is%20Not%20Valid
      (return "" false))))

(fn GetTargetActor
  (bind _target (Variables|Default|GetTarget))
  (Utilities|IsValid _target
    (:Is%20Valid
      (return _target true))
    (:Is%20Not%20Valid
      (return 0 false))))

(fn GetAttackRange
  (return 0.0))

(fn GetAttackRangeforAbilityTag
  (params (AbilityTag :type Gameplay%20Tag%20Structure))
  (return 0.0))