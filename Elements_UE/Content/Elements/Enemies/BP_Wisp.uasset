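; Wisp enemy actor that drags a linked skeletal mesh actor (OtherMesh) behind it and feeds that mesh to a Niagara effect.
; BeginPlay binds OtherMesh's skeletal mesh component to the Niagara "Mesh" user variable.
; Each Tick eases OtherMesh toward the wisp's location, using RotateSpeed as the interpolation speed, and points its X axis away from the wisp.
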(event EventBeginPlay
  (bind _othermesh (Variables|Default|GetOtherMesh)
    (:then
      (Class|NiagaraFunctionLibrary|OverrideSystemUserVariableSkeletalMeshComponent (Variables|Default|GetNiagara) "Mesh" (Variables|/Script/Engine.SkeletalMeshActor|GetSkeletalMeshComponent _othermesh)))
    (:else)))

(event Collision|EventActorBeginOverlap
  (params (OtherActor :type Actor%20Object%20Reference)))

(event EventTick
  (params (DeltaSeconds :type Float%20%28single-precision%29))
  (bind _returnvalue (Transformation|GetActorLocation))
  (bind _othermesh (Variables|Default|GetOtherMesh)
    (:then
      (Transformation|SetActorLocation _othermesh (Math|Interpolation|VInterpTo (Transformation|GetActorLocation _othermesh) _returnvalue DeltaSeconds (Variables|Default|GetRotate%20Speed)) false true)
      (Transformation|SetActorRotation (Variables|Default|GetOtherMesh) (Math|Rotator|MakeRotfromX (- (Transformation|GetActorLocation _othermesh) _returnvalue)) true))
    (:else)))

(fn ConstructionScript
  (|CallParentFunction))