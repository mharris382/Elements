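; BP_TestEnemyMage is a test mage enemy character that colors its mesh and Niagara effects to match its CharacterElementTag.
; The construction script tints the mesh and sets the effect color directly, using a manual lookup.
; BeginPlay waits briefly, then applies the element again to the dynamic material and Niagara components.
; It returns its AttackRange variable for attack range queries but zero for any per-ability range query.
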(event EventBeginPlay
  (bind _characterelementtag (Variables|Default|GetCharacterElementTag))
  (|CallParentFunction)
  (Utilities|FlowControl|Delay 0.2)
  (Default|SetMeshandElement (Variables|Default|GetBP_DynamicMaterialElement) _characterelementtag (Variables|Character|GetMesh) "Tint" false)
  (Default|SetElement (Variables|Default|GetBP_ElementalNiagaraSystem) _characterelementtag))

(event Collision|EventActorBeginOverlap
  (params (OtherActor :type Actor%20Object%20Reference))
  (|CallParentFunction OtherActor))

(event EventTick
  (params (DeltaSeconds :type Float%20%28single-precision%29))
  (|CallParentFunction DeltaSeconds))

(fn ConstructionScript
  (bind _characterelementtag (Variables|Default|GetCharacterElementTag))
  (|CallParentFunction)
  (Default|SetMeshandElement (Variables|Default|GetBP_DynamicMaterialElement) _characterelementtag (Variables|Character|GetMesh) "Tint" true)
  (Default|SetElementColorDirect (Variables|Default|GetBP_ElementalNiagaraSystem) _characterelementtag))

(fn GetAttackRange
  (return (Variables|Default|GetAttack%20Range)))

(fn GetAttackRangeforAbilityTag
  (params (AbilityTag :type Gameplay%20Tag%20Structure))
  (return 0.0))