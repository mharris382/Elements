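; BP_DummyEnemy is a dummy enemy that displays its ability system health on a health bar.
; The construction script creates a dynamic material instance for the bar and previews it half full.
; From BeginPlay, a looping timer polls Health and Max Health from the Ability System Component, prints an error if either is missing, and sets the material's fill parameter to their ratio.
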(event Custom|Update%20HealthBar
  (bind _hardrefabilitysystemcomponent (Variables|Default|GetHardRefAbilitySystemComponent))
  (bind _hardrefabilitysystemcomponent_2 (Variables|Default|GetHardRefAbilitySystemComponent))
  (bind (_bsuccessfullyfoundattribute _returnvalue) (Ability|Attribute|GetFloatAttributefromAbilitySystemComponent _hardrefabilitysystemcomponent "(AttributeName=\"MaxHealth\",Attribute=/Script/Elements_UE.AttributeSetBase:MaxHealth,AttributeOwner=\"/Script/CoreUObject.Class'/Script/Elements_UE.AttributeSetBase'\")"))
  (bind (_bsuccessfullyfoundattribute_2 _returnvalue_2) (Ability|Attribute|GetFloatAttributefromAbilitySystemComponent _hardrefabilitysystemcomponent_2 "(AttributeName=\"Health\",Attribute=/Script/Elements_UE.AttributeSetBase:Health,AttributeOwner=\"/Script/CoreUObject.Class'/Script/Elements_UE.AttributeSetBase'\")"))
  (Utilities|IsValid _hardrefabilitysystemcomponent_2
    (:Is%20Valid
      (Utilities|CheckforAttributeNotFoundError _bsuccessfullyfoundattribute_2 "Health")
      (Utilities|CheckforAttributeNotFoundError _bsuccessfullyfoundattribute "Max Health")
      (CallFunction|UpdateHealthBar _returnvalue_2 _returnvalue))))

(event EventBeginPlay
  (|CallParentFunction)
  (Utilities|Time|SetTimerbyEvent (delegate Custom|Update%20HealthBar) 0.1 true))

(event Collision|EventActorBeginOverlap
  (params (OtherActor :type Actor%20Object%20Reference)))

(event EventTick
  (params (DeltaSeconds :type Float%20%28single-precision%29)))

(fn ConstructionScript
  (bind _returnvalue (Rendering|Material|CreateDynamicMaterialInstance (Variables|Default|GetHealthBar) 0 "/Game/Elements/Materials/UI/MI_TestHealthBar.MI_TestHealthBar" "None" :!class /Script/Engine.PrimitiveComponent))
  (Variables|Default|SetTestHealthBarMaterial _returnvalue)
  (CallFunction|UpdateHealthBar 5e+01 1e+02))

(fn UpdateHealthBar
  (params (Health :type Float%20%28double-precision%29) (MaxHealth :type Float%20%28double-precision%29))
  (Rendering|Material|SetScalarParameterValue (Variables|Default|GetTestHealthBarMaterial) "Fill Percent" (/ Health MaxHealth) :!class /Script/Engine.MaterialInstanceDynamic))