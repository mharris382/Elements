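; BP_WispBase is a base wisp enemy Blueprint with a Niagara effect tinted by element color data.
; On BeginPlay it loops over every DT_ElementData row and writes each ElementColorID to the ElementColor parameter of NSWispEnemy.
; The loop does not filter by the wisp's element, so the last row found sets the final color.
; A GetCharacterElement node sits unconnected, and Tick and overlap events are disabled.
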(event EventBeginPlay
  (|CallParentFunction)
  (bind _outrownames (DataTable|GetDataTableRowNames "/Game/Data/DT_ElementData.DT_ElementData"))
  (for _array_element _outrownames
    (bind _returnvalue (Utilities|GetDataTableRow "/Game/Data/DT_ElementData.DT_ElementData" _array_element)
      (:then
        (Niagara|SetNiagaraVariable(LinearColor) (Variables|Default|GetNS_WispEnemy) "ElementColor" (.ElementColorID (Utilities|Struct|BreakElementData _returnvalue)))))))

(event Collision|EventActorBeginOverlap
  (params (OtherActor :type Actor%20Object%20Reference))
  (|CallParentFunction OtherActor) ; This node is disabled and will not be called.\nDrag off pins to build functionality.
)

(event EventTick
  (params (DeltaSeconds :type Float%20%28single-precision%29))
  (|CallParentFunction DeltaSeconds) ; This node is disabled and will not be called.\nDrag off pins to build functionality.
)

(fn ConstructionScript
  (|CallParentFunction))